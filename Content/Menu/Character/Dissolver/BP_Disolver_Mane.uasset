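; Menu character actor that plays a dissolve effect on a skeletal mesh with matching Niagara particles when play begins.
; A setup macro, run at construction and again at BeginPlay, pushes Alpha, edge color and dissolve texture to the SKSkelet system and mesh, creating dynamic material instances per slot.
; A timeline then drives Alpha on both mesh and particles together.
; A parallel static mesh setup exists but never runs.
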(event `self.ReceiveBeginPlay`
  (`self.Updat Date SK`))

(event `Updat Date SK`
  (`self.SKMesh_Setup` (`self.SK_Skelet`) (`self.SkeletalMesh`)
    (:`Completed`
      (bind (_direction _newtrack_0) (`Timeline|Timeline` :!via `PlayFromStart`)
        (:`Update`
          (`MeshComponent.SetScalarParameterValueOnMaterials` (`self.SkeletalMesh`) "Alpha" _newtrack_0)
          (`NiagaraComponent.SetVariableFloat` (`self.SK_Skelet`) "Alpha" _newtrack_0))))))

(fn `UserConstructionScript`
  (`self.SKMesh_Setup` (`self.SK_Skelet`) (`self.SkeletalMesh`)))